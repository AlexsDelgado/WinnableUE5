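; BP_Bollard is a bollard whose Cylinder component rises and sinks between a lowered and a raised position.
; MoveUp and MoveDown set the IsUp flag and animate the cylinder with MoveComponentTo over a short, fixed time.
; Toggle picks the opposite move from IsUp, while RandomUp, despite its name, runs that same toggle when a random roll falls within ChanceOfChange.
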(event `Move Up`
  (set `self.IsUp` true :!label _label)
  (`KismetSystemLibrary.MoveComponentTo` (`self.Cylinder`) (0.0 0.0 300.0) (struct) false false 0.8))

(event `RandomUp`
  (if (<= (`KismetMathLibrary.RandomInteger` 101) (`self.Chance of Change`))
    (if (`self.IsUp`) :!label _label_2
      (set `self.IsUp` false :!label _label_3)
      (`KismetSystemLibrary.MoveComponentTo` (`self.Cylinder`) (0.0 0.0 0.0) (struct) false false 0.8)
      (else
        (goto _label)))))

(event `Toggle`
  (goto _label_2))

(event `Move Down`
  (goto _label_3))

(fn `UserConstructionScript`)