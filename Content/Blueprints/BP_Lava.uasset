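; BP_Lava is a lava actor whose own movement logic is obsolete, since a note says the level Blueprint now moves it.
; The leftover, disconnected graph offsets the actor in the XZ plane by platform angle, speed and a multiplier, with both offsets currently multiplied by zero.
; Other unused fragments toggle that multiplier for when the player climbs too high and accelerate speed after a delay.
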(fn `UserConstructionScript`)