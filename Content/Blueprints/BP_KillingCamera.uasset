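; Kill volume actor that destroys players who overlap it and updates the two-player score.
; On begin overlap it checks the other actor's tag, Player or PlayerBP1, then destroys that actor.
; It then calls P1ScoreUp or P2ScoreUp respectively on BP_MyGameplayInstance.
; The Box hit event is empty, and a similar disconnected copy of the logic never runs.
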(event `self.ReceiveActorBeginOverlap`
  (params (OtherActor :type "Actor Object Reference"))
  (if (`self.ActorHasTag` OtherActor "Player")
    (`self.K2_DestroyActor` OtherActor)
    (bind _asbp_my_gameplay_instance (cast `/Game/BP_MyGameplayInstance` (`GameplayStatics.GetGameInstance`)))
    (`/Game/BP_MyGameplayInstance.P1 score up` _asbp_my_gameplay_instance)
    (elif (`self.ActorHasTag` OtherActor "PlayerBP1")
      (`KismetSystemLibrary.PrintText` "Choco al pj 1" false false)
      (`self.K2_DestroyActor` OtherActor)
      (bind _asbp_my_gameplay_instance_2 (cast `/Game/BP_MyGameplayInstance` (`GameplayStatics.GetGameInstance`)))
      (`/Game/BP_MyGameplayInstance.P2 score up` _asbp_my_gameplay_instance_2))))

(event `self.Box.OnComponentHit`
  (params (HitComponent :type "PrimitiveComponent Object Reference") (OtherActor :type "Actor Object Reference") (OtherComp :type "PrimitiveComponent Object Reference") (NormalImpulse :type "Vector Structure") (Hit :type "HitResult Structure (by ref)")))

(fn `UserConstructionScript`)