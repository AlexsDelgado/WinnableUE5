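; BP_ColectarGolden is a pickup that awards its Value in points to one of two players on touch, then plays a sound and destroys itself.
; At BeginPlay it caches the first BP_Collectable in the level, which receives the points.
; The box overlap checks the actor's class, crediting P1 for BP_ThirdPersonCharacter and P2 for BP_PLAYER4.
; A DoOnce precedes that check, so any first overlap, even a non-player, uses it up.
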(event `self.ReceiveBeginPlay`
  (bind _outactors (`GameplayStatics.GetAllActorsOfClass` "/Game/Collectable/BP/BP_Collectable.BP_Collectable_C"))
  (set `self.Collectable` (`|GetArrayItem` _outactors)))

(event `self.Box.OnComponentBeginOverlap`
  (params (OverlappedComponent :type "PrimitiveComponent Object Reference") (OtherActor :type "Actor Object Reference") (OtherComp :type "PrimitiveComponent Object Reference") (OtherBodyIndex :type Integer) (bFromSweep :type Boolean) (SweepResult :type "HitResult Structure (by ref)"))
  (bind _value (`self.Value`))
  (bind _collectable (`self.Collectable`))
  (`/Engine/EditorBlueprintResources/StandardMacros.DoOnce` false
    (:`Completed`
      (if (`KismetMathLibrary.ClassIsChildOf` (`GameplayStatics.GetObjectClass` OtherActor) "/Game/ThirdPerson/Blueprints/BP_ThirdPersonCharacter.BP_ThirdPersonCharacter_C")
        (`/Game/Collectable/BP/BP_Collectable.AddPoint P1` _collectable _value)
        (`GameplayStatics.PlaySound2D` "/Game/Sounds/SFX/Objeto-recolectado.Objeto-recolectado" 1.0 1.0 0.0 null null :!label _label)
        (`self.K2_DestroyActor`)
        (elif (`KismetMathLibrary.ClassIsChildOf` (`GameplayStatics.GetObjectClass` OtherActor) "/Game/ThirdPerson/Blueprints/BP_PLAYER4.BP_PLAYER4_C")
          (`/Game/Collectable/BP/BP_Collectable.Add Points P2` _collectable _value)
          (goto _label))))))

(fn `UserConstructionScript`)