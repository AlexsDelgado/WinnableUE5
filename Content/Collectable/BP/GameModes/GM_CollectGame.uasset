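; GM_CollectGame is the game mode for a timed collection game, tracking score, level, object count and game-over state.
; StartGame, run on BeginPlay and RestartGame, resets score, count and countdown, then sets the Clock timer that flags game over at zero.
; ObjectCollected awards level-scaled points and periodically raises the capped level.
; SpawnItem, not called here, spawns actors at random BP_SpawnPoint locations, destroying each used point.
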(event `self.ReceiveBeginPlay`
  (`self.StartGame`))

(event `RestartGame`
  ;[1 1 1] Restart Game Module
  (`self.StartGame`))

(event `Clock`
  (bind _output_get (set `self.Time` (- (`self.Time`) 1)))
  (if (== _output_get 0)
    (set `self.GameOver` true)
    (`KismetSystemLibrary.K2_ClearTimer` null "Clock")))

(fn `GetGameMode`)

(fn `ObjectCollected`
  (set `self.Score` (+ (`self.Score`) (* (`self.Level`) 10)))
  (set `self.ObjectCount` (+ (`self.ObjectCount`) 1))
  (if (== (mod (`self.ObjectCount`) 5) 0)
    (set `self.Level` (`KismetMathLibrary.Min` (+ (`self.Level`) 1) 5))))

(fn `SpawnItem`
  (locals (LocalSpawnReferences :type "Array of /Game/Collectable/BP/BP_SpawnPoint Object Reference") (LocalItem :type "/Game/Collectable/BP/BP_SpawnPoint Object Reference"))
  (bind _outactors (`GameplayStatics.GetAllActorsOfClass` "/Game/Collectable/BP/BP_SpawnPoint.BP_SpawnPoint_C"))
  (set `local.LocalSpawnReferences` _outactors)
  (for _ (range 7)
    (set `local.LocalItem` (`KismetArrayLibrary.Array_Random` (`local.LocalSpawnReferences`)))
    (`|SpawnActorFromClass` "/Game/Collectable/BP/BP_Object.BP_Object_C" (`KismetMathLibrary.MakeTransform` (`self.K2_GetActorLocation` (`local.LocalItem`))) "AdjustIfPossibleButAlwaysSpawn" "MultiplyWithRoot" null null)
    (`KismetArrayLibrary.Array_RemoveItem` (`local.LocalSpawnReferences`) (`local.LocalItem`))
    (`self.K2_DestroyActor` (`local.LocalItem`))))

(fn `UserConstructionScript`)