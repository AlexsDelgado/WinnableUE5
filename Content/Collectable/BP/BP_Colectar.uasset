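; BP_Colectar is a pickup actor that awards points to one of two player characters and then destroys itself.
; On BeginPlay it caches the first BP_Collectable in the level, which receives the points.
; Every Box overlap plays a pickup sound, then a DoOnce gate casts the actor to BP_ThirdPersonCharacter (P1) or BP_PLAYER4 (P2).
; A successful cast adds that player's points and plays a collected sound before destruction.
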(event `self.ReceiveBeginPlay`
  (bind _outactors (`GameplayStatics.GetAllActorsOfClass` "/Game/Collectable/BP/BP_Collectable.BP_Collectable_C"))
  (set `self.Collectable` (`|GetArrayItem` _outactors)))

(event `self.Box.OnComponentBeginOverlap`
  (params (OverlappedComponent :type "PrimitiveComponent Object Reference") (OtherActor :type "Actor Object Reference") (OtherComp :type "PrimitiveComponent Object Reference") (OtherBodyIndex :type Integer) (bFromSweep :type Boolean) (SweepResult :type "HitResult Structure (by ref)"))
  (bind _collectable (`self.Collectable`))
  (`GameplayStatics.PlaySound2D` "/Game/Sounds/Pickup_2.Pickup_2" 1.0 1.0 0.0 null null)
  (`/Engine/EditorBlueprintResources/StandardMacros.DoOnce` false
    (:`Completed`
      (cast `/Game/ThirdPerson/Blueprints/BP_ThirdPersonCharacter` OtherActor
        (:`then`
          (`/Game/Collectable/BP/BP_Collectable.AddPoint P1` _collectable))
        (:`CastFailed`
          (cast `/Game/ThirdPerson/Blueprints/BP_PLAYER4` OtherActor)
          (`/Game/Collectable/BP/BP_Collectable.AddPointsP2` _collectable)))
      (`GameplayStatics.PlaySound2D` "/Game/Sounds/SFX/Objeto-recolectado.Objeto-recolectado" 1.0 1.0 0.0 null null)
      (`self.K2_DestroyActor`))))

(fn `UserConstructionScript`)