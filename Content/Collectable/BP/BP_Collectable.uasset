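; BP_Collectable runs a timed two-player collection round, tracking points and updating the BP_WidgetScore HUD.
; Each point added spawns the next BP_Colectar at a random BP_SpawnPoint.
; A looping one-second timer counts down, then credits the leader through BP_MyGameplayInstance.
; A tie plays a sudden-death sound, leaving SpawnObject to credit the winner when the next point lands.
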(event `self.ReceiveBeginPlay`
  (bind _returnvalue (`|CreateWidget` "/Game/Collectable/BP/BP_WidgetScore.BP_WidgetScore_C"))
  (bind _output_get (set `self.Widget` _returnvalue))
  (`UserWidget.AddToViewport` _output_get 0)
  (`KismetSystemLibrary.K2_SetTimer` null "CountDown" 1.0 true)
  (`KismetSystemLibrary.Delay` 0.2)
  (`self.SpawnObject`))

(event `SpawnObject`
  (bind _outactors (`GameplayStatics.GetAllActorsOfClass` "/Game/Collectable/BP/BP_SpawnPoint.BP_SpawnPoint_C"))
  (`|SpawnActorFromClass` "/Game/Collectable/BP/BP_Colectar.BP_Colectar_C" (`self.GetTransform` (`|GetArrayItem` _outactors (`KismetMathLibrary.RandomIntegerInRange` 0 (`KismetArrayLibrary.Array_LastIndex` _outactors)))) "AdjustIfPossibleButAlwaysSpawn" "MultiplyWithRoot" null null)
  (if (<= (`self.Time`) 0)
    (if (< (`self.Points P1`) (`self.Points P2`))
      (bind _asbp_my_gameplay_instance (cast `/Game/BP_MyGameplayInstance` (`GameplayStatics.GetGameInstance`)))
      (`/Game/BP_MyGameplayInstance.P2 score up` _asbp_my_gameplay_instance)
      (else
        (bind _asbp_my_gameplay_instance_2 (cast `/Game/BP_MyGameplayInstance` (`GameplayStatics.GetGameInstance`)))
        (`/Game/BP_MyGameplayInstance.P1 score up` _asbp_my_gameplay_instance_2)))))

(event `CountDown`
  (bind _points_p2 (`self.Points P2`))
  (bind _points_p1 (`self.Points P1`))
  (bind _output_get (set `self.Time` (- (`self.Time`) 1)))
  (`/Game/Collectable/BP/BP_WidgetScore.Time Update` (`self.Widget`) _output_get)
  (if (== (`self.Time`) 0)
    (if (== _points_p2 _points_p1)
      (`GameplayStatics.PlaySound2D` "/Game/Sounds/SFX/Muerte_súbita.Muerte_súbita" 1.0 1.0 0.0 null null)
      (set `TextBlock.Text` "0!" (`/Game/Collectable/BP/BP_WidgetScore.Countdown` (`self.Widget`)))
      (elif (< _points_p1 _points_p2)
        (bind _asbp_my_gameplay_instance (cast `/Game/BP_MyGameplayInstance` (`GameplayStatics.GetGameInstance`)))
        (`/Game/BP_MyGameplayInstance.P2 score up` _asbp_my_gameplay_instance)
        (else
          (bind _asbp_my_gameplay_instance_2 (cast `/Game/BP_MyGameplayInstance` (`GameplayStatics.GetGameInstance`)))
          (`/Game/BP_MyGameplayInstance.P1 score up` _asbp_my_gameplay_instance_2))))
    (`KismetSystemLibrary.K2_ClearTimer` null "CountDown")))

(fn `AddPoint P1`
  (bind _output_get (set `self.Points P1` (+ (`self.Points P1`) 1)))
  (`/Game/Collectable/BP/BP_WidgetScore.T1` (`self.Widget`) _output_get)
  (`self.SpawnObject`))

(fn `AddPointsP2`
  (bind _output_get (set `self.Points P2` (+ (`self.Points P2`) 1)))
  (`/Game/Collectable/BP/BP_WidgetScore.T2` (`self.Widget`) _output_get)
  (`self.SpawnObject`))

(fn `UserConstructionScript`)