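; Game Instance for a two-player obstacle run game that keeps both players' scores and the score widget.
; On Init, after a short delay, it creates the score widget once and adds it to the viewport.
; Each score event increments that player, updates the widget and shows a round-win screen, or, if the score is already three, shows a game-win screen and resets both scores.
; Either outcome pauses the game.
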(event `self.ReceiveInit`
  (`KismetSystemLibrary.Delay` 0.1)
  (if (`self.Is UI Created`)
    (`UserWidget.AddToViewport` (`self.Score UI`) 0)
    (else
      (bind _returnvalue (`|CreateWidget` "/Game/UI/UIW_Score.UIW_Score_C"))
      (bind _output_get (set `self.Score UI` _returnvalue))
      (`UserWidget.AddToViewport` _output_get 0)
      (set `self.Is UI Created` true))))

(event `P1 score up`
  (bind _p1score (`self.P1Score`))
  ;[1 1 1] Sistema de puntos
  (if (== _p1score 3)
    (bind _returnvalue (`|CreateWidget` "/Game/UI/UIW_P1GameWin.UIW_P1GameWin_C"))
    (`UserWidget.AddToViewport` _returnvalue 0)
    (`self.reset score`)
    (`GameplayStatics.SetGamePaused` true)
    (else
      (`/Engine/EditorBlueprintResources/StandardMacros.IncrementInt` _p1score
        (:`  `
          (`/Game/UI/UIW_Score.IncreaseP1Score` (`self.Score UI`))
          (bind _returnvalue_2 (`|CreateWidget` "/Game/UI/UIW_P1Win.UIW_P1Win_C"))
          (`UserWidget.AddToViewport` _returnvalue_2 0)
          (`GameplayStatics.SetGamePaused` true))))))

(event `P2 score up`
  (bind _p2score (`self.P2Score`))
  ;[1 1 1] Sistema de puntos
  (if (== _p2score 3)
    (bind _returnvalue (`|CreateWidget` "/Game/UI/UIW_P2GameWin.UIW_P2GameWin_C"))
    (`UserWidget.AddToViewport` _returnvalue 0)
    (`self.reset score`)
    (`GameplayStatics.SetGamePaused` true)
    (else
      (`/Engine/EditorBlueprintResources/StandardMacros.IncrementInt` _p2score
        (:`  `
          (`/Game/UI/UIW_Score.IncreaseP2Score` (`self.Score UI`))
          (bind _returnvalue_2 (`|CreateWidget` "/Game/UI/UIW_P2Win.UIW_P2Win_C"))
          (`UserWidget.AddToViewport` _returnvalue_2 0)
          (`GameplayStatics.SetGamePaused` true))))))

(event `reset score`
  (set `self.P2Score` 0)
  (set `self.P1Score` 0))